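; NormalDoorInOutside_BP is a door actor that the player opens by pressing E while near it.
; Overlapping the Trigger enables player input and shows HelpfulText only if the door's yaw is under 10 degrees; leaving disables input and hides the text.
; E plays the DoorRotate timeline forward, which sets the actor's absolute yaw each update, with no reverse to close it.
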(event `self.Trigger.OnComponentBeginOverlap`
  (params (OverlappedComponent :type "PrimitiveComponent Object Reference") (OtherActor :type "Actor Object Reference") (OtherComp :type "PrimitiveComponent Object Reference") (OtherBodyIndex :type Integer) (bFromSweep :type Boolean) (SweepResult :type "HitResult Structure (by ref)"))
  (bind (_returnvalue_roll _returnvalue_pitch _returnvalue_yaw) (`KismetMathLibrary.BreakRotator` (`self.K2_GetActorRotation` self)))
  ;[1 1 1] Tigger, enable input and show helpful text
  (`self.EnableInput` (`GameplayStatics.GetPlayerController` 0))
  (`SceneComponent.SetVisibility` (`self.Helpful Text`) (> 10.0 _returnvalue_yaw) false))

(event `self.Trigger.OnComponentEndOverlap`
  (params (OverlappedComponent :type "PrimitiveComponent Object Reference") (OtherActor :type "Actor Object Reference") (OtherComp :type "PrimitiveComponent Object Reference") (OtherBodyIndex :type Integer))
  ;[1 1 1] Tigger, enable input and show helpful text
  (`self.DisableInput` (`GameplayStatics.GetPlayerController` 0))
  (`SceneComponent.SetVisibility` (`self.Helpful Text`) (`self.False`) false))

(event `Key|E`
  (params (Key :type "Key Structure"))
  ;[1 1 1] Press E to Move Door
  (:`Pressed`
    (bind (_direction _rotate) (`Timeline|DoorRotate`)
      (:`Update`
        (`self.K2_SetActorRotation` self (`KismetMathLibrary.MakeRotator` 0.0 0.0 (.z _rotate)) false)))))

(fn `UserConstructionScript`)