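; Template pickup actor that the first-person player collects into the HUD inventory while inside its trigger.
; The construction script fills the ItemInfo struct and sets the mesh from custom variables.
; Trigger overlaps toggle the prompt widget and in-range flag, gating a handler bound to the character's PickupItem dispatcher.
; Pickup adds ItemInfo, refreshes the inventory, sets EquipmentID, and hides the actor with collision disabled rather than destroying it.
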(event `self.ReceiveBeginPlay`
  (bind _iteminfo (`self.ItemInfo`))
  (bind _pickuptextreference (`self.PickupTextReference`))
  (bind (_item _itemimage _pickuptext _itemid) (break `/Game/han/Blueprint/UI/ItemInfoStruct` _iteminfo))
  ;[1 1 1] Event Begin Play
  (bind _returnvalue (`|CreateWidget` "/Game/han/Blueprint/UI/PickupText.PickupText_C"))
  (set `self.PickupTextReference` _returnvalue)
  (setmembers `/Game/han/Blueprint/UI/ItemInfoStruct` :`StructRef` _iteminfo :`Item` self)
  (set `/Game/han/Blueprint/UI/PickupText.PickupActor` _item _pickuptextreference)
  (set `/Game/han/Blueprint/UI/PickupText.PickupText` _pickuptext _pickuptextreference)
  (bind _asfirst_person_character_custom (cast `/Game/han/Blueprint/FirstPersonCharacterCustom` (`GameplayStatics.GetPlayerCharacter` 0)))
  (bind _output_get (set `self.CharacterReference` _asfirst_person_character_custom))
  (add `/Game/han/Blueprint/FirstPersonCharacterCustom.PickupItem` _output_get (delegate `PickupItem_Event_0`)))

(event `self.Trigger.OnComponentBeginOverlap`
  (params (OverlappedComponent :type "PrimitiveComponent Object Reference") (OtherActor :type "Actor Object Reference") (OtherComp :type "PrimitiveComponent Object Reference") (OtherBodyIndex :type Integer) (bFromSweep :type Boolean) (SweepResult :type "HitResult Structure (by ref)"))
  ;[1 1 1] Overlap Trigger Event
  (cast `/Game/han/Blueprint/FirstPersonCharacterCustom` OtherActor)
  (`UserWidget.AddToViewport` (`self.PickupTextReference`) 0)
  (set `self.IsInRange?` true))

(event `PickupItem_Event_0`
  (bind _gameuhditemreference (`/Game/han/Blueprint/FirstPersonCharacterCustom.GameUHDItemReference` (`self.CharacterReference`)))
  ;[1 1 1] Pickup and add data
  (if (and (`self.GetActorEnableCollision`) (`self.IsInRange?`))
    (`KismetArrayLibrary.Array_Add` (`/Game/han/Blueprint/UI/GameHUDItem.Inventory` _gameuhditemreference) (`self.ItemInfo`))
    (`Widget.RemoveFromParent` (`self.PickupTextReference`))
    (`self.SetActorHiddenInGame` true)
    (`self.SetActorEnableCollision` false)
    (`/Game/han/Blueprint/UI/GameHUDItem.RefreshInventory` _gameuhditemreference)
    (set `/Game/han/Blueprint/UI/GameHUDItem.EquipmentID` (`.ItemID_12_BE7F59354AB43A790478AB8254F0D094` (break `/Game/han/Blueprint/UI/ItemInfoStruct` (`self.ItemInfo`))) _gameuhditemreference)))

(event `self.Trigger.OnComponentEndOverlap`
  (params (OverlappedComponent :type "PrimitiveComponent Object Reference") (OtherActor :type "Actor Object Reference") (OtherComp :type "PrimitiveComponent Object Reference") (OtherBodyIndex :type Integer))
  ;[1 1 1] Overlap Trigger Event
  (cast `/Game/han/Blueprint/FirstPersonCharacterCustom` OtherActor)
  (`Widget.RemoveFromParent` (`self.PickupTextReference`))
  (set `self.IsInRange?` false))

(fn `UserConstructionScript`
  (setmembers `/Game/han/Blueprint/UI/ItemInfoStruct` :`StructRef` (`self.ItemInfo`) :`Item` self :`ItemImage` (`self.CustomImage`) :`PickupText` (`self.CustomPickupText`) :`ItemID` (`self.ItemID`))
  (`StaticMeshComponent.SetStaticMesh` (`self.StaticMesh`) (`self.CustomStaticMesh`)))