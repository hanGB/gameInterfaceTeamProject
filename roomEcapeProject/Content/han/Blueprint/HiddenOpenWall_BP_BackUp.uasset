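; Hidden wall actor, apparently a backup copy, that opens while something overlaps its Trigger component.
; On overlap begin, two timelines play: WallMovement offsets the location from the position saved at BeginPlay, and WallRotate sets the pitch.
; The rotation is absolute, with roll and yaw forced to zero.
; On overlap end, both timelines reverse to close the wall, with no filter on the overlapping actor.
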(event `self.ReceiveBeginPlay`
  ;[1 1 1] Get Initial Location
  (set `self.InitialDoorLocation` (`self.K2_GetActorLocation` self)))

(event `self.Trigger.OnComponentBeginOverlap`
  (params (OverlappedComponent :type "PrimitiveComponent Object Reference") (OtherActor :type "Actor Object Reference") (OtherComp :type "PrimitiveComponent Object Reference") (OtherBodyIndex :type Integer) (bFromSweep :type Boolean) (SweepResult :type "HitResult Structure (by ref)"))
  ;[1 1 1] Tigger, Move the Wall
  (`|ExecutionSequence`
    (:`then_0`
      (bind (_direction _movement) (`Timeline|WallMovement` :!label _label)
        (:`Update`
          (`self.K2_SetActorLocation` self (+ _movement (`self.InitialDoorLocation`)) false false))))
    (:`then_1`
      (bind (_direction_2 _rotate) (`Timeline|WallRotate` :!label _label_2)
        (:`Update`
          (`self.K2_SetActorRotation` self (`KismetMathLibrary.MakeRotator` 0.0 (.y _rotate)) false))))))

(event `self.Trigger.OnComponentEndOverlap`
  (params (OverlappedComponent :type "PrimitiveComponent Object Reference") (OtherActor :type "Actor Object Reference") (OtherComp :type "PrimitiveComponent Object Reference") (OtherBodyIndex :type Integer))
  ;[1 1 1] Tigger, Move the Wall
  (`|ExecutionSequence`
    (:`then_0`
      (goto _label :!via `Reverse`))
    (:`then_1`
      (goto _label_2 :!via `Reverse`))))

(fn `UserConstructionScript`)