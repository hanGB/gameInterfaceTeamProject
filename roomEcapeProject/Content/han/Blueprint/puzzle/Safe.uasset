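; Keypad safe puzzle actor that opens on a correct code and yields an inventory item.
; A trigger overlap enables input and toggles the keypad display, while number keys build a code of up to four digits.
; Enter, F or Multiply checks it against Answer, playing the SafeMovement timeline or flashing an error.
; Once open, E adds the item to the player's HUD inventory, sets its equipment ID and reverses the movement.
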(event `self.ReceiveBeginPlay`
  ;[1 1 1] Make Numbers Array and Set Initial Location
  (set `self.Numbers` (`|MakeArray` (`self.num2`) (`self.num5`) (`self.num6`) (`self.num9`) (`self.num10`) (`self.num11`) (`self.num4`) (`self.num7`) (`self.num12`) (`self.num14`) (`self.num13`) (`self.num15`)))
  (set `self.InitialSafeLocation` (`self.K2_GetActorLocation` self))
  (bind _asfirst_person_character_custom (cast `/Game/han/Blueprint/FirstPersonCharacterCustom` (`GameplayStatics.GetPlayerCharacter` 0)))
  (set `self.CharacterReference` _asfirst_person_character_custom))

(event `Key|Zero`
  (params (Key :type "Key Structure"))
  ;[1 1 1] Input Number to inputNum
  (:`Pressed`
    (if (< (`KismetStringLibrary.Len` (`KismetTextLibrary.Conv_TextToString` (`self.inputNum`))) 4)
      (set `self.inputNum` (`KismetTextLibrary.Conv_StringToText` (`KismetStringLibrary.Concat_StrStr` (`KismetTextLibrary.Conv_TextToString` (`self.inputNum`)) "0")))
      (`TextRenderComponent.K2_SetText` (`self.number`) (`self.inputNum`)))))

(event `Key|Six`
  (params (Key :type "Key Structure"))
  ;[1 1 1] Input Number to inputNum
  (:`Pressed`
    (if (< (`KismetStringLibrary.Len` (`KismetTextLibrary.Conv_TextToString` (`self.inputNum`))) 4)
      (set `self.inputNum` (`KismetTextLibrary.Conv_StringToText` (`KismetStringLibrary.Concat_StrStr` (`KismetTextLibrary.Conv_TextToString` (`self.inputNum`)) "6")))
      (`TextRenderComponent.K2_SetText` (`self.number`) (`self.inputNum`)))))

(event `Key|One`
  (params (Key :type "Key Structure"))
  ;[1 1 1] Input Number to inputNum
  (:`Pressed`
    (if (< (`KismetStringLibrary.Len` (`KismetTextLibrary.Conv_TextToString` (`self.inputNum`))) 4)
      (set `self.inputNum` (`KismetTextLibrary.Conv_StringToText` (`KismetStringLibrary.Concat_StrStr` (`KismetTextLibrary.Conv_TextToString` (`self.inputNum`)) "1")))
      (`TextRenderComponent.K2_SetText` (`self.number`) (`self.inputNum`)))))

(event `Key|Seven`
  (params (Key :type "Key Structure"))
  ;[1 1 1] Input Number to inputNum
  (:`Pressed`
    (if (< (`KismetStringLibrary.Len` (`KismetTextLibrary.Conv_TextToString` (`self.inputNum`))) 4)
      (set `self.inputNum` (`KismetTextLibrary.Conv_StringToText` (`KismetStringLibrary.Concat_StrStr` (`KismetTextLibrary.Conv_TextToString` (`self.inputNum`)) "7")))
      (`TextRenderComponent.K2_SetText` (`self.number`) (`self.inputNum`)))))

(event `Key|E`
  (params (Key :type "Key Structure"))
  (bind _item_info (`self.Item Info`))
  (bind _gameuhditemreference (`/Game/han/Blueprint/FirstPersonCharacterCustom.GameUHDItemReference` (`self.CharacterReference`)))
  ;[1 1 1] Pickup and add data
  (:`Pressed`
    (if (and (`self.GetActorEnableCollision`) (`self.IsInRange?`) (`self.isOpened`) (not (`self.getCard?`)))
      (`KismetArrayLibrary.Array_Add` (`/Game/han/Blueprint/UI/GameHUDItem.Inventory` _gameuhditemreference) _item_info)
      (`|ExecutionSequence`
        (:`then_0`
          ;[1 1 1] Event Press Enter
          (bind (_direction _movement) (`Timeline|SafeMovement` :!via `Reverse` :!label _label)
            (:`Update`
              (`self.K2_SetActorLocation` self (+ _movement (`self.InitialSafeLocation`)) false false))))
        (:`then_1`
          (set `self.getCard?` true)
          (`/Game/han/Blueprint/UI/GameHUDItem.RefreshInventory` _gameuhditemreference)
          (set `/Game/han/Blueprint/UI/GameHUDItem.EquipmentID` (`.ItemID_12_BE7F59354AB43A790478AB8254F0D094` (break `/Game/han/Blueprint/UI/ItemInfoStruct` _item_info)) _gameuhditemreference))))))

(event `Key|Two`
  (params (Key :type "Key Structure"))
  ;[1 1 1] Input Number to inputNum
  (:`Pressed`
    (if (< (`KismetStringLibrary.Len` (`KismetTextLibrary.Conv_TextToString` (`self.inputNum`))) 4)
      (set `self.inputNum` (`KismetTextLibrary.Conv_StringToText` (`KismetStringLibrary.Concat_StrStr` (`KismetTextLibrary.Conv_TextToString` (`self.inputNum`)) "2")))
      (`TextRenderComponent.K2_SetText` (`self.number`) (`self.inputNum`)))))

(event `Key|Eight`
  (params (Key :type "Key Structure"))
  ;[1 1 1] Input Number to inputNum
  (:`Pressed`
    (if (< (`KismetStringLibrary.Len` (`KismetTextLibrary.Conv_TextToString` (`self.inputNum`))) 4)
      (set `self.inputNum` (`KismetTextLibrary.Conv_StringToText` (`KismetStringLibrary.Concat_StrStr` (`KismetTextLibrary.Conv_TextToString` (`self.inputNum`)) "8")))
      (`TextRenderComponent.K2_SetText` (`self.number`) (`self.inputNum`)))))

(event `Key|Multiply`
  (params (Key :type "Key Structure"))
  ;[1 1 1] Event Press Enter
  (:`Pressed`
    (if (`KismetTextLibrary.EqualEqual_TextText` (`self.inputNum`) (`self.answer`)) :!label _label_2
      (`|ExecutionSequence`
        (:`then_0`
          (set `self.isOpened` true)
          (`SceneComponent.SetVisibility` (`self.useText`) true false))
        (:`then_1`
          (goto _label)))
      (else
        (set `self.inputNum` "")
        (`SceneComponent.SetVisibility` (`self.Error`) true false)
        (`KismetSystemLibrary.Delay` 1.0)
        (`SceneComponent.SetVisibility` (`self.Error`) false false)))))

(event `Key|Enter`
  (params (Key :type "Key Structure"))
  ;[1 1 1] Event Press Enter
  (:`Pressed`
    (goto _label_2)))

(event `Key|F`
  (params (Key :type "Key Structure"))
  ;[1 1 1] Event Press Enter
  (:`Pressed`
    (goto _label_2)))

(event `Key|Three`
  (params (Key :type "Key Structure"))
  ;[1 1 1] Input Number to inputNum
  (:`Pressed`
    (if (< (`KismetStringLibrary.Len` (`KismetTextLibrary.Conv_TextToString` (`self.inputNum`))) 4)
      (set `self.inputNum` (`KismetTextLibrary.Conv_StringToText` (`KismetStringLibrary.Concat_StrStr` (`KismetTextLibrary.Conv_TextToString` (`self.inputNum`)) "3")))
      (`TextRenderComponent.K2_SetText` (`self.number`) (`self.inputNum`)))))

(event `Key|Nine`
  (params (Key :type "Key Structure"))
  ;[1 1 1] Input Number to inputNum
  (:`Pressed`
    (if (< (`KismetStringLibrary.Len` (`KismetTextLibrary.Conv_TextToString` (`self.inputNum`))) 4)
      (set `self.inputNum` (`KismetTextLibrary.Conv_StringToText` (`KismetStringLibrary.Concat_StrStr` (`KismetTextLibrary.Conv_TextToString` (`self.inputNum`)) "9")))
      (`TextRenderComponent.K2_SetText` (`self.number`) (`self.inputNum`)))))

(event `self.Trigger.OnComponentBeginOverlap`
  (params (OverlappedComponent :type "PrimitiveComponent Object Reference") (OtherActor :type "Actor Object Reference") (OtherComp :type "PrimitiveComponent Object Reference") (OtherBodyIndex :type Integer) (bFromSweep :type Boolean) (SweepResult :type "HitResult Structure (by ref)"))
  ;[1 1 1] Event Trigger Overlap
  (`self.EnableInput` (`GameplayStatics.GetPlayerController` 0))
  (if (`self.isOpened`)
    (set `self.IsInRange?` true)
    (`SceneComponent.SetVisibility` (`self.useText`) true false)
    (else
      (`|ExecutionSequence`
        (:`then_0`
          (`SceneComponent.ToggleVisibility` (`self.Numbers`) false))
        (:`then_1`
          (`SceneComponent.ToggleVisibility` (`self.number`) false))))))

(event `self.ReceiveTick`
  (params (DeltaSeconds :type "Float (single-precision)"))
  ;[1 1 1] Off Number After Opened
  (if (`self.isOpened`)
    (`|ExecutionSequence`
      (:`then_0`
        (`SceneComponent.SetVisibility` (`self.number`) false false))
      (:`then_1`
        (`SceneComponent.SetVisibility` (`self.Numbers`) false false))
      (:`then_2`
        (if (`self.getCard?`)
          (`SceneComponent.SetVisibility` (`self.useText`) false false))))))

(event `Key|Four`
  (params (Key :type "Key Structure"))
  ;[1 1 1] Input Number to inputNum
  (:`Pressed`
    (if (< (`KismetStringLibrary.Len` (`KismetTextLibrary.Conv_TextToString` (`self.inputNum`))) 4)
      (set `self.inputNum` (`KismetTextLibrary.Conv_StringToText` (`KismetStringLibrary.Concat_StrStr` (`KismetTextLibrary.Conv_TextToString` (`self.inputNum`)) "4")))
      (`TextRenderComponent.K2_SetText` (`self.number`) (`self.inputNum`)))))

(event `self.Trigger.OnComponentEndOverlap`
  (params (OverlappedComponent :type "PrimitiveComponent Object Reference") (OtherActor :type "Actor Object Reference") (OtherComp :type "PrimitiveComponent Object Reference") (OtherBodyIndex :type Integer))
  ;[1 1 1] Event Trigger Overlap
  (`self.DisableInput` (`GameplayStatics.GetPlayerController` 0))
  (if (`self.isOpened`)
    (set `self.IsInRange?` false)
    (`SceneComponent.SetVisibility` (`self.useText`) false false)
    (else
      (`|ExecutionSequence`
        (:`then_0`
          (`SceneComponent.ToggleVisibility` (`self.Numbers`) false))
        (:`then_1`
          (`SceneComponent.ToggleVisibility` (`self.number`) false))))))

(event `Key|Five`
  (params (Key :type "Key Structure"))
  ;[1 1 1] Input Number to inputNum
  (:`Pressed`
    (if (< (`KismetStringLibrary.Len` (`KismetTextLibrary.Conv_TextToString` (`self.inputNum`))) 4)
      (set `self.inputNum` (`KismetTextLibrary.Conv_StringToText` (`KismetStringLibrary.Concat_StrStr` (`KismetTextLibrary.Conv_TextToString` (`self.inputNum`)) "5")))
      (`TextRenderComponent.K2_SetText` (`self.number`) (`self.inputNum`)))))

(fn `UserConstructionScript`)